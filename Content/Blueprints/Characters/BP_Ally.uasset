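; BP_Ally is an ally character Blueprint that emits footstep noise events for AI hearing while it moves.
; A looping timer started on BeginPlay checks whether the summed X and Y velocity is non-zero, then calls PawnMakeNoise at the actor's location.
; Loudness is a fixed low value when crouching, otherwise the ratio of current max walk speed to the DataAsset's sprint speed.
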(event `self.ReceiveBeginPlay`
  ;[1 1 1] FootstepsSound
  (`parent.ReceiveBeginPlay`)
  (`KismetSystemLibrary.K2_SetTimerDelegate` (delegate `Footstep`) 0.3 true))

(event `Footstep`
  (bind (_returnvalue_x _returnvalue_y) (`KismetMathLibrary.BreakVector` (`self.GetVelocity`)))
  (bind _charactermovement (`self.CharacterMovement`))
  ;[1 1 1] FootstepsSound
  (if (!= (+ _returnvalue_x _returnvalue_y) 0.0)
    (`self.PawnMakeNoise` (`KismetMathLibrary.SelectFloat` 0.3 (/ (`CharacterMovementComponent.MaxWalkSpeed` _charactermovement) (`/Game/_managers/DataAsset/BP/BP_DataAsset.sprintSpeed` (`self.dataAsset`))) (`NavMovementComponent.IsCrouching` _charactermovement)) (`self.K2_GetActorLocation`) true self)))

(fn `UserConstructionScript`
  (`parent.UserConstructionScript`))