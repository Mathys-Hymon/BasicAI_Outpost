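; BP_Player is a player Blueprint that handles smooth aim-down-sights for a camera and weapon.
; Pressing IA_Aim plays the SmoothAim timeline, which blends the camera field of view and the weapon's relative Y location between base and aiming values, and releasing it reverses the blend.
; The Ping event is empty, and the construction script only calls its parent.
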(event `/Game/Blueprints/BPI/BPI_Player.Ping`)

(event `EnhancedInput|/Game/_managers/Inputs/IA_Aim`
  (params (ActionValue :type Boolean) (ElapsedSeconds :type "Float (double-precision)") (TriggeredSeconds :type "Float (double-precision)") (InputAction :type "InputAction Object Reference" :default "/Game/_managers/Inputs/IA_Aim.IA_Aim"))
  (bind _weapon (`self.Weapon`))
  (bind (_relativelocation_x _relativelocation_y _relativelocation_z) (`KismetMathLibrary.BreakVector` (`SceneComponent.RelativeLocation` _weapon)))
  (:`Started`
    (bind (_direction _aimingtimeline) (`Timeline|SmoothAim` :!label _label)
      (:`Update`
        (`CameraComponent.SetFieldOfView` (`self.Camera`) (`KismetMathLibrary.Lerp` (`self.BaseFOV`) (`self.AimingFOV`) _aimingtimeline))
        (`SceneComponent.K2_SetRelativeLocation` _weapon (`KismetMathLibrary.MakeVector` _relativelocation_x (`KismetMathLibrary.Lerp` (`self.BaseWeaponLocation`) (`self.AimingWeaponLocation`) _aimingtimeline) _relativelocation_z) false false))))
  (:`Completed`
    (goto _label :!via `Reverse`)))

(fn `UserConstructionScript`
  (`parent.UserConstructionScript`))