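; Base character Blueprint handling movement stances, shooting, damage and healing, with tuning read from a DataAsset.
; Aim, sprint and crouch events swap walk speed and cancel conflicting states, while a timeline resizes the capsule for crouching.
; Shoot line-traces for pawns along the controller's forward vector and calls ApplyDamage on hits.
; Damage lowers Life and calls Die at zero, while Heal spends a limited charge to restore MaxLife.
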(event `self.ReceivePossessed`
  (params (NewController :type "Controller Object Reference"))
  ;[1 1 1] BeginPlay
  (set `CharacterMovementComponent.MaxWalkSpeedCrouched` (`/Game/_managers/DataAsset/BP/BP_DataAsset.crouchSpeed` (`self.dataAsset`)) (`self.CharacterMovement`))
  (set `self.life` (`/Game/_managers/DataAsset/BP/BP_DataAsset.life` (`self.dataAsset`))))

(event `/Game/Blueprints/BPI/BPI_Player.Aim`
  ;[1 1 1] Aim
  (`/Game/Blueprints/BPI/BPI_Player.StopSprinting`)
  (set `CharacterMovementComponent.MaxWalkSpeed` (`/Game/_managers/DataAsset/BP/BP_DataAsset.aimSpeed` (`self.dataAsset`)) (`self.CharacterMovement`)))

(event `/Game/Blueprints/BPI/BPI_Player.Sprint`
  ;[1 1 1] SwitchSprint
  (`/Game/Blueprints/BPI/BPI_Player.EndCrouch`)
  (`/Game/Blueprints/BPI/BPI_Player.StopAiming`)
  (set `CharacterMovementComponent.MaxWalkSpeed` (`/Game/_managers/DataAsset/BP/BP_DataAsset.sprintSpeed` (`self.dataAsset`)) (`self.CharacterMovement`)))

(event `/Game/Blueprints/BPI/BPI_Player.StopAiming`
  ;[1 1 1] Aim
  (set `CharacterMovementComponent.MaxWalkSpeed` (`/Game/_managers/DataAsset/BP/BP_DataAsset.walkSpeed` (`self.dataAsset`)) (`self.CharacterMovement`)))

(event `/Game/Blueprints/BPI/BPI_Player.StopSprinting`
  ;[1 1 1] SwitchSprint
  (set `CharacterMovementComponent.MaxWalkSpeed` (`/Game/_managers/DataAsset/BP/BP_DataAsset.walkSpeed` (`self.dataAsset`)) (`self.CharacterMovement`)))

(event `/Game/Blueprints/BPI/BPI_Player.Shoot`
  (bind _returnvalue (`self.K2_GetActorLocation`))
  ;[1 1 1] Shoot
  (bind (_outhit _returnvalue_2) (`KismetSystemLibrary.LineTraceSingleForObjects` (+ _returnvalue (0.0 0.0 45.0)) (+ (+ _returnvalue (* (`self.GetActorForwardVector` (`self.GetController`)) (`/Game/_managers/DataAsset/BP/BP_DataAsset.shootRange` (`self.dataAsset`)))) (0.0 0.0 45.0)) (`|MakeArray` "ObjectTypeQuery3" :!type "EObjectTypeQuery Enum") false (`|MakeArray` (`self.actorToIgnoreShoot`)) "ForDuration"))
  (if _returnvalue_2
    (`GameplayStatics.ApplyDamage` (`.HitActor` (`GameplayStatics.BreakHitResult` _outhit)))))

(event `/Game/Blueprints/BPI/BPI_Player.StartCrouch`
  ;[1 1 1] Crouch
  (`/Game/Blueprints/BPI/BPI_Player.StopSprinting`)
  (`self.Crouch`)
  (set `CharacterMovementComponent.MaxWalkSpeed` (`/Game/_managers/DataAsset/BP/BP_DataAsset.crouchSpeed` (`self.dataAsset`)) (`self.CharacterMovement`))
  (bind (_direction _lerp) (`Timeline|changeCapsuleSize` :!label _label)
    (:`Update`
      (`CapsuleComponent.SetCapsuleHalfHeight` (`self.CapsuleComponent`) (`KismetMathLibrary.Lerp` 88.0 44.0 _lerp) true))))

(event `self.ReceiveAnyDamage`
  (params (Damage :type "Float (single-precision)") (DamageType :type "DamageType Object Reference") (InstigatedBy :type "Controller Object Reference") (DamageCauser :type "Actor Object Reference"))
  ;[1 1 1] Take damage
  (bind _output_get (set `self.life` (- (`self.life`) Damage)))
  (if (<= _output_get 0.0)
    (`/Game/Blueprints/BPI/BPI_Player.Die`)))

(event `/Game/Blueprints/BPI/BPI_Player.EndCrouch`
  ;[1 1 1] Crouch
  (`self.UnCrouch`)
  (set `CharacterMovementComponent.MaxWalkSpeed` (`/Game/_managers/DataAsset/BP/BP_DataAsset.walkSpeed` (`self.dataAsset`)) (`self.CharacterMovement`))
  (goto _label :!via `Reverse`))

(event `/Game/Blueprints/BPI/BPI_Player.Heal`
  ;[1 1 1] Heal
  (if (> (`self.healLeft`) 0.0)
    (set `self.healLeft` (- (`self.healLeft`) 1.0))
    (set `self.life` (`self.maxLife`))))

(fn `UserConstructionScript`)